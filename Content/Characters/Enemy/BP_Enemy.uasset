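; BP_Enemy is an enemy character Blueprint with a floating health bar widget that turns to face the player.
; On BeginPlay it casts the HealthBar0 widget to WBP_FloatingHealthBar and sets itself as the owning character.
; Every Tick it billboards the bar by setting its world rotation to a look-at toward the first player's camera location.
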(event EventBeginPlay
  (|CallParentFunction)
  (CallFunction|InitHealthBar0))

(event EventTick
  (params (DeltaSeconds :type Float%20%28single-precision%29))
  (|CallParentFunction DeltaSeconds)
  (CallFunction|UpdateHealthBar0))

(fn ConstructionScript
  (|CallParentFunction))

(fn InitHealthBar0
  (bind _aswbp_floating_health_bar (Utilities|Casting|CastToWBP_FloatingHealthBar (UserInterface|GetWidget (Variables|Default|GetHealthBar_0))))
  (Default|SetOwningCharacter _aswbp_floating_health_bar self))

(fn UpdateHealthBar0
  (bind _returnvalue (Game|GetPlayerCameraManager 0))
  (bind _healthbar_0 (Variables|Default|GetHealthBar_0))
  (bind _returnvalue_2 (Camera|GetCameraLocation _returnvalue))
  (bind _returnvalue_3 (Transformation|GetWorldLocation _healthbar_0))
  (bind _returnvalue_4 (Math|Rotator|FindLookatRotation _returnvalue_3 _returnvalue_2))
  (Transformation|SetWorldRotation _healthbar_0 (Math|Rotator|MakeRotator (.roll _returnvalue_4) (.pitch _returnvalue_4) (.yaw _returnvalue_4)) false false))