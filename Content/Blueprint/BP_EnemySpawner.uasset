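; Enemy spawner actor that keeps up to MaxSpawn enemies alive within SpawnRadius, previewed by a debug sphere in the construction script.
; A randomized one-shot timer restarts after each spawn until the limit is reached, and again when a tracked enemy is destroyed.
; Each spawn picks a random reachable point, creates the enemy facing the spawner's center, then spawns an AI controller to possess it.
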(event EventBeginPlay
  (CallFunction|StartSpawnerTimer))

(fn ConstructionScript
  (Rendering|Debug|FlushPersistentDebugLines)
  (Rendering|Debug|DrawDebugSphere (Transformation|GetActorLocation) (Variables|Default|GetSpawnRadius) 12 "(R=0.421827,G=0.000000,B=0.770833,A=1.000000)" 1e+04))

(fn SpawnEnemy
  (params (Center :type Vector))
  (if (not (CallFunction|IsSpawnLimitReached))
    (bind _newenemy (CallFunction|SpawnEnemyInternal Center))
    (Utilities|IsValid _newenemy
      (:Is%20Valid
        (Utilities|Array|AddUnique (Variables|Default|GetSpawnActors) _newenemy)))
    (else
      (Development|PrintText (Utilities|Text|FormatText "Maximum spawnable actors reached NumSpawn{Num}: MaxSpawn={Max}" (Utilities|Array|Length (Variables|Default|GetSpawnActors)) (Variables|Default|GetMaxSpawn))))))

(fn OnCharacterDestroyed
  (params (DestroyedActor :type Actor%20Object%20Reference))
  (bind _spawnactors (Variables|Default|GetSpawnActors))
  (if (Utilities|Array|ContainsItem _spawnactors DestroyedActor)
    (Utilities|Array|RemoveItem _spawnactors DestroyedActor)
    (CallFunction|StartSpawnerTimer)))

(fn RandomSpawnTime
  (bind _spawnwindowvariant (Variables|Default|GetSpawnWindowVariant))
  (return (+ (Variables|Default|GetSpawnWindow) (Math|Random|RandomFloatinRange (* _spawnwindowvariant -1.0) _spawnwindowvariant))))

(fn IsSpawnLimitReached
  (return (== (Variables|Default|GetMaxSpawn) (Utilities|Array|Length (Variables|Default|GetSpawnActors)))))

(fn CanSpawn
  (return (and (not (CallFunction|IsSpawnLimitReached)) (not (Utilities|Time|IsTimerActivebyHandle (Variables|Default|GetSpawnTimerHandle))))))

(fn OnSpawnTimerEnded
  (CallFunction|SpawnEnemy (Transformation|GetActorLocation))
  (Utilities|Time|ClearandInvalidateTimerbyHandle (Variables|Default|GetSpawnTimerHandle))
  (CallFunction|StartSpawnerTimer))

(fn StartSpawnerTimer
  (if (CallFunction|CanSpawn)
    (bind _output_get (LocalVariables|SetSpawnTime (CallFunction|RandomSpawnTime)))
    (bind _returnvalue (Utilities|Time|SetTimerbyFunctionName 0 "OnSpawnTimerEnded" _output_get))
    (Variables|Default|SetSpawnTimerHandle _returnvalue)
    (Development|PrintText (Utilities|Text|FormatText "Next enemy to be spawned in {Time} seconds" (LocalVariables|GetSpawnTime)))))

(fn SpawnEnemyInternal
  (params (Center :type Vector))
  (Utilities|FlowControl|Sequence
    (:then_0
      (|RandomizeSpawnLocation Center))
    (:then_1
      (|SpawnTheCharacter))
    (:then_2
      (|SpawnTheAI))
    (:then_3
      (return (LocalVariables|GetSpawnedEnemy)))))